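; BP_MoveableMeshActor is a mesh actor that exposes its engine events to the RuntimeBPConstructor of the runtime Blueprint system.
; On BeginPlay it binds overlap, hit, sleep and wake delegates on every primitive component under the root.
; Those component events, plus Tick, EndPlay and actor-level hit and overlap events, are passed straight to the constructor's matching Call functions.
; The actor holds no gameplay logic of its own.
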(event Custom|OnComponentBeginOverlap
  (params (OverlappedComponent :type Primitive%20Component%20Object%20Reference) (OtherActor :type Actor%20Object%20Reference) (OtherComp :type Primitive%20Component%20Object%20Reference) (OtherBodyIndex :type Integer) (bFromSweep :type Boolean) (SweepResult :type Hit%20Result%20Structure%20%28by%20ref%29))
  ;[1 1 1] Bind Events to RuntimeBPs
  (Class|RuntimeBpConstructor|CallonComponentBeginOverlap (Variables|Default|GetRuntimeBPConstructor) OverlappedComponent OtherActor OtherComp OtherBodyIndex bFromSweep SweepResult))

(event Custom|OnComponentEndOverlap
  (params (OverlappedComponent :type Primitive%20Component%20Object%20Reference) (OtherActor :type Actor%20Object%20Reference) (OtherComp :type Primitive%20Component%20Object%20Reference) (OtherBodyIndex :type Integer))
  ;[1 1 1] Bind Events to RuntimeBPs
  (Class|RuntimeBpConstructor|CallonComponentEndOverlap (Variables|Default|GetRuntimeBPConstructor) OverlappedComponent OtherActor OtherComp OtherBodyIndex))

(event Custom|OnComponentHit
  (params (HitComponent :type Primitive%20Component%20Object%20Reference) (OtherActor :type Actor%20Object%20Reference) (OtherComp :type Primitive%20Component%20Object%20Reference) (NormalImpulse :type Vector) (Hit :type Hit%20Result%20Structure%20%28by%20ref%29))
  ;[1 1 1] Bind Events to RuntimeBPs
  (Class|RuntimeBpConstructor|CallonComponentHit (Variables|Default|GetRuntimeBPConstructor) HitComponent OtherActor OtherComp NormalImpulse Hit))

(event Custom|OnComponentWake
  (params (WakingComponent :type Primitive%20Component%20Object%20Reference) (BoneName :type Name))
  ;[1 1 1] Bind Events to RuntimeBPs
  (Class|RuntimeBpConstructor|CallonComponentWake (Variables|Default|GetRuntimeBPConstructor) WakingComponent BoneName))

(event Custom|OnComponentSleep
  (params (SleepingComponent :type Primitive%20Component%20Object%20Reference) (BoneName :type Name))
  ;[1 1 1] Bind Events to RuntimeBPs
  (Class|RuntimeBpConstructor|CallonComponentSleep (Variables|Default|GetRuntimeBPConstructor) SleepingComponent BoneName))

(event Custom|BindEventsForComponent
  (params (Target :type Primitive%20Component%20Object%20Reference))
  ;[1 1 1] Bind Events to RuntimeBPs
  (Collision|AssignOnComponentBeginOverlap Target (delegate Custom|OnComponentBeginOverlap))
  (Collision|AssignOnComponentEndOverlap Target (delegate Custom|OnComponentEndOverlap))
  (Collision|AssignOnComponentHit Target (delegate Custom|OnComponentHit))
  (EventDispatchers|AssignOnComponentSleep Target (delegate Custom|OnComponentSleep))
  (EventDispatchers|AssignOnComponentWake Target (delegate Custom|OnComponentWake)))

(event Collision|EventActorEndOverlap
  (params (OtherActor :type Actor%20Object%20Reference))
  ;[1 1 1] Bind Events to RuntimeBPs
  (Class|RuntimeBpConstructor|CallonActorEndOverlap (Variables|Default|GetRuntimeBPConstructor) OtherActor))

(event Collision|EventHit
  (params (MyComp :type Primitive%20Component%20Object%20Reference) (Other :type Actor%20Object%20Reference) (OtherComp :type Primitive%20Component%20Object%20Reference) (bSelfMoved :type Boolean) (HitLocation :type Vector :default "0, 0, 0") (HitNormal :type Vector :default "0, 0, 0") (NormalImpulse :type Vector :default "0, 0, 0") (Hit :type Hit%20Result%20Structure%20%28by%20ref%29))
  ;[1 1 1] Bind Events to RuntimeBPs
  (Class|RuntimeBpConstructor|CallonEventHit (Variables|Default|GetRuntimeBPConstructor) MyComp Other OtherComp bSelfMoved HitLocation HitNormal NormalImpulse Hit))

(event EventBeginPlay
  ;[1 1 1] Bind Events to RuntimeBPs
  (for _array_element (Components|GetChildrenComponents (Variables|Transformation|GetRootComponent) true)
    (bind _asprimitive_component (Utilities|Casting|CastToPrimitiveComponent _array_element))
    (CallFunction|BindEventsforComponent _asprimitive_component)))

(event EventTick
  (params (DeltaSeconds :type Float%20%28single-precision%29))
  ;[1 1 1] Bind Events to RuntimeBPs
  (Class|RuntimeBpConstructor|CallTick (Variables|Default|GetRuntimeBPConstructor) DeltaSeconds))

(event Collision|EventActorBeginOverlap
  (params (OtherActor :type Actor%20Object%20Reference))
  ;[1 1 1] Bind Events to RuntimeBPs
  (Class|RuntimeBpConstructor|CallonActorBeginOverlap (Variables|Default|GetRuntimeBPConstructor) OtherActor))

(event EventEndPlay
  (params (EndPlayReason :type EEndPlayReason%20Enum :default "Destroyed"))
  ;[1 1 1] Bind Events to RuntimeBPs
  (Class|RuntimeBpConstructor|CallEndPlay (Variables|Default|GetRuntimeBPConstructor)))

(fn ConstructionScript)