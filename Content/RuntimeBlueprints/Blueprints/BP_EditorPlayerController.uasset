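; Player controller for the runtime Blueprint editor, hosting the BPEditorGraph widget with UI-only input.
; BeginPlay creates the graph and shows stat unit; ClearEditorGraph recreates it and loads a given save.
; ApplyUndo rebuilds rather than edits: it converts the undo stack entry to JSON and recreates its nodes in a fresh widget that replaces the old one.
; The P key resets the play widget switcher and refocuses the editor.
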(event Custom|ClearEditorGraph
  (params (LoadFile :type String))
  (bind _self self)
  (Variables|Default|SetScriptToLoad LoadFile)
  (bind _foundwidgets (Widget|GetAllWidgetsOfClass "/Game/RuntimeBlueprints/Widgets/BPEditorGraph.BPEditorGraph_C" true))
  (Widget|RemovefromParent _foundwidgets)
  (Variables|Default|SetEditorGraph 0)
  (bind _returnvalue (UserInterface|CreateWidget "/Game/RuntimeBlueprints/Widgets/BPEditorGraph.BPEditorGraph_C" _self))
  (Variables|Default|SetEditorGraph _returnvalue)
  (UserInterface|Viewport|AddtoPlayerScreen _returnvalue)
  (Variables|Default|SetbShowMouseCursor true)
  (Input|SetInputModeUIOnly _self _returnvalue "LockOnCapture")
  (Default|LoadPendingSave (Variables|Default|GetEditorGraph) (Variables|Default|GetScriptToLoad)))

(event Custom|ApplyUndo
  (params (Index :type Integer))
  (bind _scriptundostack (Variables|Default|GetScriptUndoStack))
  (bind _output (Utilities|Array|Get(acopy) _scriptundostack Index))
  (bind (_savedformat _undonodeindices) (Utilities|Struct|BreakST_UndoInfo _output))
  (bind (_jsonstring _returnvalue) (Class|RuntimeBpJsonLibrary|ScripttoJsonString _savedformat false))
  (if _returnvalue
    (Variables|Default|SetCurrentUndoIndex Index)
    (bind _returnvalue_2 (UserInterface|CreateWidget "/Game/RuntimeBlueprints/Widgets/BPEditorGraph.BPEditorGraph_C" self false))
    (Default|TransferEditorGraphInfo (Variables|Default|GetEditorGraph) _returnvalue_2)
    (Widget|RemovefromParent (Variables|Default|GetEditorGraph))
    (bind _output_get (Variables|Default|SetEditorGraph _returnvalue_2))
    (Default|CreateNodesfromJson _output_get _jsonstring false _undonodeindices)
    (Input|SetInputModeUIOnly self _output_get "LockOnCapture")
    (UserInterface|Viewport|AddtoPlayerScreen _output_get)))

(event EventBeginPlay
  (bind _self self)
  (Utilities|FlowControl|Sequence
    (:then_0
      (bind _returnvalue (UserInterface|CreateWidget "/Game/RuntimeBlueprints/Widgets/BPEditorGraph.BPEditorGraph_C" _self))
      (Variables|Default|SetEditorGraph _returnvalue)
      (UserInterface|Viewport|AddtoPlayerScreen _returnvalue)
      (Variables|Default|SetbShowMouseCursor true)
      (Input|SetInputModeUIOnly _self _returnvalue "LockOnCapture")
      (Default|LoadPendingSave (Variables|Default|GetEditorGraph) (Variables|Default|GetScriptToLoad)))
    (:then_1
      (Development|ExecuteConsoleCommand "stat unit" _self))))

(event Input|KeyboardEvents|P
  (params (Key :type Key%20Structure :default "None"))
  (bind _self self)
  (bind _editorgraph (Variables|Default|GetEditorGraph))
  (:Pressed
    (Class|WidgetSwitcher|SetActiveWidgetIndex (Variables|/Game/RuntimeBlueprints/Widgets/BPEditorGraph.BPEditorGraph_C|GetPlayWidgetSwitcher _editorgraph))
    (Input|SetInputModeUIOnly _self _editorgraph "LockOnCapture")
    (Variables|/Script/Engine.PlayerController|SetbShowMouseCursor _self true)))

(fn ConstructionScript)